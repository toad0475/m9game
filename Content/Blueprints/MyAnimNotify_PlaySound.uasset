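; Animation notify Blueprint that, despite its PlaySound name, runs a debug ground probe and plays no sound itself.
; On notify, it traces 100 units down on Visibility from the ball_l bone, passing an actor-space location as the trace start.
; The trace draws persistently and its result is unused; a default PrintString follows, then the parent notify runs.
; The name and trigger-weight overrides only forward to the parent.
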(fn `GetDefaultTriggerWeightThreshold`
  (returns (ReturnValue :type "Float (single-precision)"))
  (bind _returnvalue (`parent.GetDefaultTriggerWeightThreshold`))
  (return _returnvalue))

(fn `GetNotifyName`
  (returns (ReturnValue :type String))
  (bind _returnvalue (`parent.GetNotifyName`))
  (return _returnvalue))

(fn `Received_Notify`
  (params (MeshComp :type "SkeletalMeshComponent Object Reference") (Animation :type "AnimSequenceBase Object Reference") (EventReference :type "AnimNotifyEventReference Structure (by ref)"))
  (returns (ReturnValue :type Boolean))
  (bind _returnvalue_location (`KismetMathLibrary.BreakTransform` (`SkinnedMeshComponent.GetBoneTransform` MeshComp (`SkinnedMeshComponent.GetSocketBoneName` MeshComp "ball_l") "RTS_Actor")))
  (`KismetSystemLibrary.LineTraceSingle` :`Start` _returnvalue_location :`End` (+ _returnvalue_location (0.0 0.0 -100.0)) :`TraceChannel` "TraceTypeQuery1" :`DrawDebugType` "Persistent")
  (`KismetSystemLibrary.PrintString` "Hello")
  (bind _returnvalue (`parent.Received_Notify` MeshComp Animation EventReference))
  (return _returnvalue))